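; GenericMinion is a base minion character that the player can freeze in place with an ability.
; On BeginPlay it caches BP_Player and sizes its capsule tall and narrow for Minion instances, short and wide otherwise.
; Tick polls the E key, zeroing walk speed while held if the UIhealth ability timer is nonzero.
; Without E held, a Delay on Tick raises walk speed in periodic steps with no cap.
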(event Collision|EventActorBeginOverlap
  (params (OtherActor :type Actor%20Object%20Reference)))

(event EventTick
  (params (DeltaSeconds :type Float%20%28single-precision%29))
  (bind _charactermovement (Variables|Character|GetCharacterMovement))
  (if (Game|Player|IsInputKeyDown (Game|GetPlayerController 0) "E")
    (if (not (== 0.0 (Variables|/Game/BlockBreaker/Blueprints/UiHealth.UiHealth_C|GetAbiltytimer (Variables|/Game/BlockBreaker/Blueprints/BP_Player.BP_Player_C|GetUIhealth (Variables|Default|Getplayer)))))
      (Variables|/Script/Engine.CharacterMovementComponent|SetMaxWalkSpeed _charactermovement 0.0))
    (else
      (Utilities|FlowControl|Delay 0.2)
      (Variables|/Script/Engine.CharacterMovementComponent|SetMaxWalkSpeed _charactermovement (+ (Variables|/Script/Engine.CharacterMovementComponent|GetMaxWalkSpeed _charactermovement) 1e+01)))))

(event EventBeginPlay
  (bind _capsulecomponent (Variables|Collision|GetCapsuleComponent))
  (bind _asbp_player (Utilities|Casting|CastToBP_Player (Game|GetPlayerCharacter 0))
    (:then
      (Variables|Default|Setplayer _asbp_player))
    (:CastFailed
      (Development|PrintString "Hello")))
  (Utilities|Casting|CastToMinion self
    (:then
      (Components|Capsule|SetCapsuleSize _capsulecomponent 34.0 75.0 true))
    (:CastFailed
      (Components|Capsule|SetCapsuleSize _capsulecomponent 115.0 6e+01 true))))

(fn ConstructionScript)
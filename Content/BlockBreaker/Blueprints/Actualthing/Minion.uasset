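; Minion actor or pawn that takes damage and reports its death to the player's health UI.
; BeginPlay enables mesh collision, caches the player's BP_Player and runs TakeDamage, which AnyDamage also calls.
; TakeDamage subtracts damage from health clamped between zero and one; at zero it calls MinionDead on the UiHealth widget and destroys itself.
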(event EventBeginPlay
  (Collision|SetCollisionEnabled (Variables|Character|GetMesh) "QueryAndPhysics")
  (bind _asbp_player (Utilities|Casting|CastToBP_Player (Game|GetPlayerCharacter 0)))
  (CallFunction|TakeDamage (stale Game|Damage|EventAnyDamage Damage) (Variables|/Game/BlockBreaker/Blueprints/BP_Player.BP_Player_C|GetUIhealth _asbp_player)))

(event Collision|EventActorBeginOverlap
  (params (OtherActor :type Actor%20Object%20Reference)))

(event Game|Damage|EventAnyDamage
  (params (Damage :type Float%20%28single-precision%29) (DamageType :type Damage%20Type%20Object%20Reference) (InstigatedBy :type Controller%20Object%20Reference) (DamageCauser :type Actor%20Object%20Reference))
  (CallFunction|TakeDamage Damage (Variables|/Game/BlockBreaker/Blueprints/BP_Player.BP_Player_C|GetUIhealth (stale EventBeginPlay _asbp_player))))

(fn ConstructionScript)

(fn TakeDamage
  (params (Damage :type Float%20%28single-precision%29) (UserInterface :type Ui%20Health%20Object%20Reference))
  (bind _output_get (Variables|Default|SetHealth (Math|Float|Clamp(Float) (- (Variables|Default|GetHealth) Damage))))
  (if (== _output_get 0.0)
    (bind _asui_health (Utilities|Casting|CastToUiHealth UserInterface))
    (Default|MinionDead _asui_health)
    (Actor|DestroyActor)
    (return _asui_health)))

(fn NewFunction0
  (return (AI|GetBlackboard 0)))
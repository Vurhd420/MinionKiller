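; AI controller for minions in the BlockBreaker game that runs the MinionGoto behavior tree on the MIniondATA blackboard.
; On begin play, every tick and every perception update, it fills an invalid "Enemy" key with the first BP_Player in the level, regardless of what is perceived.
; TakeDamage lowers a normalized Health value and destroys this controller actor at zero.
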(event OnPerceptionUpdated(AIPerception)
  (params (UpdatedActors :type Array%20of%20Actor%20Object%20References))
  (Utilities|IsValid (AI|Components|Blackboard|GetValueasObject (stale EventBeginPlay _blackboardcomponent) (Utilities|Name|MakeLiteralName "Enemy"))
    (:Is%20Not%20Valid
      (bind _outactors (Actor|GetAllActorsOfClass "/Game/BlockBreaker/Blueprints/BP_Player.BP_Player_C"))
      (bind _asbp_player (Utilities|Casting|CastToBP_Player (Utilities|Array|Get(acopy) _outactors)))
      (AI|Components|Blackboard|SetValueasObject (stale EventBeginPlay _blackboardcomponent) (Utilities|Name|MakeLiteralName "Enemy") _asbp_player))))

(event EventBeginPlay
  (Utilities|FlowControl|Sequence
    (:then_0
      (bind _blackboardcomponent (Class|AIController|UseBlackboard "/Game/BlockBreaker/Blueprints/Actualthing/MIniondATA.MIniondATA"))
      (AI|RunBehaviorTree "/Game/BlockBreaker/Blueprints/Actualthing/MinionGoto.MinionGoto"))
    (:then_1
      (Utilities|IsValid (AI|Components|Blackboard|GetValueasObject _blackboardcomponent (Utilities|Name|MakeLiteralName "Enemy"))
        (:Is%20Not%20Valid
          (bind _outactors (Actor|GetAllActorsOfClass "/Game/BlockBreaker/Blueprints/BP_Player.BP_Player_C"))
          (bind _asbp_player (Utilities|Casting|CastToBP_Player (Utilities|Array|Get(acopy) _outactors)))
          (AI|Components|Blackboard|SetValueasObject _blackboardcomponent (Utilities|Name|MakeLiteralName "Enemy") _asbp_player))))))

(event EventTick
  (params (DeltaSeconds :type Float%20%28single-precision%29))
  (Utilities|IsValid (AI|Components|Blackboard|GetValueasObject (stale EventBeginPlay _blackboardcomponent) (Utilities|Name|MakeLiteralName "Enemy"))
    (:Is%20Not%20Valid
      (bind _outactors (Actor|GetAllActorsOfClass "/Game/BlockBreaker/Blueprints/BP_Player.BP_Player_C"))
      (bind _asbp_player (Utilities|Casting|CastToBP_Player (Utilities|Array|Get(acopy) _outactors)))
      (AI|Components|Blackboard|SetValueasObject (stale EventBeginPlay _blackboardcomponent) (Utilities|Name|MakeLiteralName "Enemy") _asbp_player))))

(fn ConstructionScript)

(fn TakeDamage
  (params (Damge :type Float%20%28single-precision%29))
  (bind _output_get (Variables|Default|SetHealth (Math|Float|Clamp(Float) (- (Variables|Default|GetHealth) Damge))))
  (if (== _output_get 0.0)
    (Actor|DestroyActor)))
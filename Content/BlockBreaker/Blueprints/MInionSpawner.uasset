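; Minion spawner for BlockBreaker that spawns enemies at randomized positions derived from the player's location.
; It spawns once on BeginPlay, then Tick feeds a Delay that paces further spawns while the player lives.
; A Rarity-scaled roll picks a regular minion, a rare big one or none, with a flag preventing consecutive big spawns.
; Each regular spawn also fires a server-launch console command, and HasHitSpot is set but never read.
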(event Custom|Playerhitspot
  (Variables|Default|SetHasHitSpot true))

(event EventBeginPlay
  (bind _asbp_player (Utilities|Casting|CastToBP_Player (Game|GetPlayerCharacter 0)))
  (if (Math|Random|RandomBool)
    (Variables|Default|SetMultiplaying 1.0)
    (else
      ;[1 1 1] Get Random Vector in range
      (Variables|Default|SetMultiplaying -1.0)))
  ;[1 1 1] Spawn BigMinion1/20
  (Math|Float|CompareFloat (Math|Conversions|ToFloat(Integer) (Math|Random|RandomIntegerinRange 0 (Math|Float|Truncate (Variables|Default|GetRarity)))) 1.0
    (:>
      (Variables|Default|SetBigMinion false :!label _label)
      (bind _returnvalue (Game|SpawnActorfromClass "/Game/BlockBreaker/Blueprints/Actualthing/Minion.Minion_C" (Math|Transform|MakeTransform (Math|Vector|MakeVector (Math|Random|RandomFloatinRange (* (+ (.x (Transformation|GetActorLocation _asbp_player)) 2e+02) (Variables|Default|GetMultiplaying)) 1e+03) (Math|Random|RandomFloatinRange (.y (Transformation|GetActorLocation _asbp_player)) 1e+03) (Math|Random|RandomFloatinRange (.z (Transformation|GetActorLocation _asbp_player)) 1e+03)) "0.000000,90.000000,0.000000" "1,1,1") "AdjustIfPossibleButAlwaysSpawn" 0 0))
      (Components|Capsule|SetCapsuleSize (Variables|/Script/Engine.Character|GetCapsuleComponent _returnvalue) 34.0 75.0 true)
      (Development|ExecuteConsoleCommand "UE4Editor.exe ProjectName MapName -server -game -log" (Game|GetPlayerController 0)))
    (:==
      (if (Variables|Default|GetBigMinion)
        (goto _label)
        (else
          (Variables|Default|SetBigMinion true)
          (bind _returnvalue_2 (Game|SpawnActorfromClass "/Game/BlockBreaker/Blueprints/Actualthing/BigMIniondup.BigMIniondup_C" (Math|Transform|MakeTransform (Math|Vector|MakeVector (Math|Random|RandomFloatinRange (* (+ (.x (Transformation|GetActorLocation _asbp_player)) 2e+02) (Variables|Default|GetMultiplaying)) 1e+03) (Math|Random|RandomFloatinRange (.y (Transformation|GetActorLocation _asbp_player)) 1e+03) (Math|Random|RandomFloatinRange (.z (Transformation|GetActorLocation _asbp_player)) 1e+03)) "0, 0, 0" "1,1,1") "Undefined" 0 0))
          (Components|Capsule|SetCapsuleSize (Variables|/Script/Engine.Character|GetCapsuleComponent _returnvalue_2) 6e+01 115.0 true))))))

(event EventTick
  (params (DeltaSeconds :type Float%20%28single-precision%29))
  (if (Variables|/Game/BlockBreaker/Blueprints/BP_Player.BP_Player_C|GetIs%20Dead (stale EventBeginPlay _asbp_player))
    (Variables|Default|SetHasHitSpot false)
    (else
      (Utilities|FlowControl|Delay (Variables|Default|GetSpawnLEngth))
      (if (Math|Random|RandomBool)
        (Variables|Default|SetMultiplaying 1.0)
        (else
          ;[1 1 1] Get Random Vector in range
          (Variables|Default|SetMultiplaying -1.0)))
      ;[1 1 1] Spawn BigMinion1/20
      (Math|Float|CompareFloat (Math|Conversions|ToFloat(Integer) (Math|Random|RandomIntegerinRange 0 (Math|Float|Truncate (Variables|Default|GetRarity)))) 1.0
        (:>
          (Variables|Default|SetBigMinion false :!label _label)
          (bind _returnvalue (Game|SpawnActorfromClass "/Game/BlockBreaker/Blueprints/Actualthing/Minion.Minion_C" (Math|Transform|MakeTransform (Math|Vector|MakeVector (Math|Random|RandomFloatinRange (* (+ (.x (Transformation|GetActorLocation (stale EventBeginPlay _asbp_player))) 2e+02) (Variables|Default|GetMultiplaying)) 1e+03) (Math|Random|RandomFloatinRange (.y (Transformation|GetActorLocation (stale EventBeginPlay _asbp_player))) 1e+03) (Math|Random|RandomFloatinRange (.z (Transformation|GetActorLocation (stale EventBeginPlay _asbp_player))) 1e+03)) "0.000000,90.000000,0.000000" "1,1,1") "AdjustIfPossibleButAlwaysSpawn" 0 0))
          (Components|Capsule|SetCapsuleSize (Variables|/Script/Engine.Character|GetCapsuleComponent _returnvalue) 34.0 75.0 true)
          (Development|ExecuteConsoleCommand "UE4Editor.exe ProjectName MapName -server -game -log" (Game|GetPlayerController 0)))
        (:==
          (if (Variables|Default|GetBigMinion)
            (goto _label)
            (else
              (Variables|Default|SetBigMinion true)
              (bind _returnvalue_2 (Game|SpawnActorfromClass "/Game/BlockBreaker/Blueprints/Actualthing/BigMIniondup.BigMIniondup_C" (Math|Transform|MakeTransform (Math|Vector|MakeVector (Math|Random|RandomFloatinRange (* (+ (.x (Transformation|GetActorLocation (stale EventBeginPlay _asbp_player))) 2e+02) (Variables|Default|GetMultiplaying)) 1e+03) (Math|Random|RandomFloatinRange (.y (Transformation|GetActorLocation (stale EventBeginPlay _asbp_player))) 1e+03) (Math|Random|RandomFloatinRange (.z (Transformation|GetActorLocation (stale EventBeginPlay _asbp_player))) 1e+03)) "0, 0, 0" "1,1,1") "Undefined" 0 0))
              (Components|Capsule|SetCapsuleSize (Variables|/Script/Engine.Character|GetCapsuleComponent _returnvalue_2) 6e+01 115.0 true))))))))

(fn ConstructionScript)
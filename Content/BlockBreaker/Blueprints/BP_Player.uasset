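; BlockBreaker's first-person player character, handling movement, rifle/shotgun combat, the HUD ability and death.
; BeginPlay creates the HUD, attaches a rifle and spawns the minion spawner; switching weapons destroys and respawns the gun.
; Shooting delegates camera-aimed shots to EquippedGun, gated by CanShoot delays, and reloads when either ammo count is empty.
; Zero-health hits hide and teleport the player behind a restart widget; Reset restores health and clears minions.
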(event Custom|Attacked
  (if (== 0.0 (Variables|Default|GetHealth))
    (Default|Deathed (stale EventBeginPlay _returnvalue))
    (CallFunction|KIll)
    (Variables|Default|SetIs%20Dead true)
    (Utilities|FlowControl|Delay 3.0)
    (else
      (Variables|Default|SetHit true)
      (Utilities|FlowControl|Delay 1.0)
      (Variables|Default|SetHit false))))

(event Custom|FinishedDeathScreen
  (CallFunction|Reset))

(event EventBeginPlay
  (bind _returnvalue (UserInterface|CreateWidget "/Game/BlockBreaker/Blueprints/UiHealth.UiHealth_C" (Game|GetPlayerController 0)))
  (UserInterface|Viewport|AddtoViewport _returnvalue 0)
  (Variables|Default|SetUIhealth _returnvalue)
  (bind _returnvalue_2 (Game|SpawnActorfromClass "/Game/BlockBreaker/Blueprints/BP_Rifle.BP_Rifle_C" (Math|Transform|MakeTransform "0, 0, 0" "0, 0, 0" "1,1,1") "Undefined" 0 0))
  (bind _output_get (Variables|Default|SetEquippedGun _returnvalue_2))
  (Variables|/Game/BlockBreaker/Blueprints/UiHealth.UiHealth_C|SetAmmo (Variables|Default|GetUIhealth) (Variables|/Game/BlockBreaker/Blueprints/BP_BaseGun.BP_BaseGun_C|GetMagazine (Variables|Default|GetEquippedGun)))
  (Transformation|AttachComponentToComponent (Variables|/Script/Engine.Actor|GetRootComponent _output_get) (Variables|Default|GetGunLocation) "None" "SnapToTarget" "SnapToTarget" "KeepRelative" true)
  (bind _returnvalue_3 (Game|SpawnActorfromClass "/Game/BlockBreaker/Blueprints/MInionSpawner.MInionSpawner_C" (Math|Transform|MakeTransform "0, 0,242.000000" "0, 0, 0" "1,1,1") "Undefined" 0 0))
  (Variables|Default|SetMinionSpawner _returnvalue_3))

(event Collision|EventActorBeginOverlap
  (params (OtherActor :type Actor%20Object%20Reference)))

(event EventTick
  (params (DeltaSeconds :type Float%20%28single-precision%29)))

(event Input|AxisEvents|InputAxisMoveForward
  (params (AxisValue :type Float%20%28single-precision%29))
  (bind _returnvalue (== AxisValue 1.0))
  (bind _returnvalue_2 (== AxisValue 3.0))
  (if (not (Variables|Default|GetIs%20Dead))
    (Utilities|SetSpeed _returnvalue_2 _returnvalue
      (:ExecOUt
        (if (Math|Boolean|ORBoolean _returnvalue_2 _returnvalue (== AxisValue -1.0))
          (Pawn|Input|AddMovementInput (Transformation|GetActorForwardVector) AxisValue false)
          (Variables|Default|SetRunning _returnvalue_2)
          (Variables|Default|SetWalking _returnvalue))))))

(event Input|AxisEvents|InputAxisEsc
  (params (AxisValue :type Float%20%28single-precision%29))
  (if (== AxisValue 1.0)
    (Default|EscClicked (Variables|Default|GetRestorat))))

(event Input|AxisEvents|InputAxisLookHorizontal
  (params (AxisValue :type Float%20%28single-precision%29))
  (if (not (Variables|Default|GetIs%20Dead))
    (Pawn|Input|AddControllerYawInput AxisValue)))

(event Input|AxisEvents|InputAxisLookVertical
  (params (AxisValue :type Float%20%28single-precision%29))
  (if (not (Variables|Default|GetIs%20Dead))
    (Pawn|Input|AddControllerPitchInput AxisValue)))

(event Input|AxisEvents|InputAxisSwitchWeapons
  (params (AxisValue :type Float%20%28single-precision%29))
  (if (Variables|Default|GetCanShoot)
    (if (== AxisValue 1.0)
      (Actor|DestroyActor (Variables|Default|GetEquippedGun))
      (bind _returnvalue (Game|SpawnActorfromClass "/Game/BlockBreaker/Blueprints/BP_Rifle.BP_Rifle_C" (Math|Transform|MakeTransform "0, 0, 0" "0, 0, 0" "1,1,1") "Undefined" 0 0))
      (bind _output_get (Variables|Default|SetEquippedGun _returnvalue))
      (Transformation|AttachComponentToComponent (Variables|/Script/Engine.Actor|GetRootComponent _output_get) (Variables|Default|GetGunLocation) "None" "SnapToTarget" "SnapToTarget" "KeepRelative" true)
      (elif (== AxisValue 2.0)
        (Actor|DestroyActor (Variables|Default|GetEquippedGun))
        (bind _returnvalue_2 (Game|SpawnActorfromClass "/Game/BlockBreaker/Blueprints/Shotgun.Shotgun_C" (Math|Transform|MakeTransform "0, 0, 0" "0, 0, 0" "1,1,1") "Undefined" 0 0))
        (bind _output_get_2 (Variables|Default|SetEquippedGun _returnvalue_2))
        (Transformation|AttachComponentToComponent (Variables|/Script/Engine.Actor|GetRootComponent _output_get_2) (Variables|Default|GetGunLocation) "None" "SnapToTarget" "SnapToTarget" "KeepRelative" true)))))

(event Input|AxisEvents|InputAxisMoveRight
  (params (AxisValue :type Float%20%28single-precision%29))
  (if (not (Variables|Default|GetIs%20Dead))
    (Pawn|Input|AddMovementInput (Transformation|GetActorRightVector) AxisValue false)))

(event Input|AxisEvents|InputAxisSpecialMovement
  (params (AxisValue :type Float%20%28single-precision%29))
  (if (== AxisValue 1.0)
    (Character|Jump)))

(event Input|AxisEvents|InputAxisShoot
  (params (AxisValue :type Float%20%28single-precision%29))
  (bind _uihealth (Variables|Default|GetUIhealth))
  (bind _equippedgun (Variables|Default|GetEquippedGun))
  (bind _equippedgun_2 (Variables|Default|GetEquippedGun))
  (bind _fpscamera (Variables|Default|GetFpscamera))
  (bind _returnvalue (Transformation|GetWorldLocation _fpscamera))
  (if (Math|Boolean|ANDBoolean (== AxisValue 1.0) (Variables|Default|GetCanShoot) (not (Variables|/Game/BlockBreaker/Blueprints/UiHealth.UiHealth_C|GetAbilityon (Variables|Default|GetUIhealth))))
    (if (or (== (Math|Conversions|ToFloat(Integer) (Variables|/Game/BlockBreaker/Blueprints/UiHealth.UiHealth_C|GetRifleAmmo _uihealth)) 0.0) (== (Math|Conversions|ToFloat(Integer) (Variables|/Game/BlockBreaker/Blueprints/UiHealth.UiHealth_C|GetShotgunAmmo _uihealth)) 0.0))
      (Variables|Default|SetCanShoot false)
      (Default|Reload _uihealth)
      (Utilities|FlowControl|Delay (+ (Variables|/Game/BlockBreaker/Blueprints/BP_BaseGun.BP_BaseGun_C|GetReload _equippedgun) 0.501))
      (Variables|Default|SetCanShoot true)
      (Variables|/Game/BlockBreaker/Blueprints/UiHealth.UiHealth_C|SetAmmo _uihealth (Variables|/Game/BlockBreaker/Blueprints/BP_BaseGun.BP_BaseGun_C|GetMagazine _equippedgun_2))
      (elif (not (Variables|Default|GetIs%20Dead))
        (if (not (Variables|Default|GetRunning))
          (Default|Shot _uihealth)
          (Utilities|Casting|CastToShotgun _equippedgun
            (:then
              _)
            (:CastFailed
              _))
          (Default|Shoot _equippedgun_2 _returnvalue (+ _returnvalue (* (Math|Vector|GetForwardVector _fpscamera) (Variables|/Game/BlockBreaker/Blueprints/BP_BaseGun.BP_BaseGun_C|GetMaxBulletDistance (Variables|Default|GetEquippedGun)))) _uihealth)
          (Variables|Default|SetCanShoot false)
          (Utilities|FlowControl|Delay (Variables|/Game/BlockBreaker/Blueprints/BP_BaseGun.BP_BaseGun_C|GetFireRate (Variables|Default|GetEquippedGun)))
          (Variables|Default|SetCanShoot true))))))

(event Input|AxisEvents|InputAxisReload
  (params (AxisValue :type Float%20%28single-precision%29))
  (bind _uihealth (Variables|Default|GetUIhealth))
  (if (== AxisValue 1.0)
    (Variables|Default|SetCanShoot false)
    (Default|Reload _uihealth)
    (Utilities|FlowControl|Delay (+ (Variables|/Game/BlockBreaker/Blueprints/BP_BaseGun.BP_BaseGun_C|GetReload (Variables|Default|GetEquippedGun)) 0.501))
    (Variables|Default|SetCanShoot true)
    (Variables|/Game/BlockBreaker/Blueprints/UiHealth.UiHealth_C|SetAmmo _uihealth (Variables|/Game/BlockBreaker/Blueprints/BP_BaseGun.BP_BaseGun_C|GetMagazine (Variables|Default|GetEquippedGun)))))

(event Input|AxisEvents|InputAxisPower
  (params (AxisValue :type Float%20%28single-precision%29))
  (bind _uihealth (Variables|Default|GetUIhealth))
  (if (== AxisValue 1.0)
    (Default|Abilty _uihealth)
    (else
      (Default|AbilityOff _uihealth))))

(fn ConstructionScript)

(fn KIll
  (bind _mesh (Variables|Character|GetMesh))
  (bind _fpscamera (Variables|Default|GetFpscamera))
  (bind _returnvalue (Transformation|GetWorldRotation _fpscamera))
  (Rendering|SetVisibility _mesh false true)
  (Collision|SetCollisionEnabled _mesh "NoCollision")
  (Rendering|SetVisibility (Variables|/Script/Engine.Actor|GetRootComponent (Variables|Default|GetEquippedGun)) false false)
  (bind _returnvalue_2 (UserInterface|CreateWidget "/Game/BlockBreaker/Blueprints/WpB_restoart.WpB_restoart_C" (Game|GetPlayerController 0)))
  (UserInterface|Viewport|AddtoViewport _returnvalue_2 0)
  (Variables|Default|SetRestorat _returnvalue_2)
  (Transformation|Teleport "0.000000, 0,242.000000" "0, 0, 0")
  (Pawn|Input|AddControllerYawInput (- 0.0 (.pitch _returnvalue)))
  (Pawn|Input|AddControllerPitchInput (- 0.0 (.yaw _returnvalue)))
  (return _returnvalue_2))

(fn Reset
  (Variables|Default|SetHealth 1e+02)
  (Variables|Default|SetIs%20Dead false)
  (Variables|/Game/BlockBreaker/Blueprints/WpB_restoart.WpB_restoart_C|SetShown (Variables|Default|GetRestorat) false)
  (bind _outactors (Actor|GetAllActorsOfClass "/Game/BlockBreaker/Blueprints/Actualthing/Minion.Minion_C"))
  (bind _outactors_2 (Actor|GetAllActorsOfClass "/Game/BlockBreaker/Blueprints/Actualthing/BigMIniondup.BigMIniondup_C"))
  (for _array_element _outactors_2
    (Actor|DestroyActor _array_element))
  (for _array_element_2 _outactors
    (Actor|DestroyActor _array_element_2))
  (Default|Reset (Variables|Default|GetUIhealth)))

(fn ShotgunShot
  (params (Start :type Vector) (ForwardVector :type Vector) (Damge :type Float%20%28single-precision%29))
  (bind _outhit (Collision|LineTraceByChannel Start ForwardVector "TraceTypeQuery1" false 0 "None"))
  (Variables|Default|SetHitLocation (.Location (Collision|BreakHitResult _outhit)))
  (Utilities|FlowControl|Sequence
    (:then_0
      (Effects|SpawnEmitteratLocation "/Game/BlockBreaker/ParticleSystems/PS_BulletImpact.PS_BulletImpact" (.Location (Collision|BreakHitResult _outhit)))
      (Game|Damage|ApplyDamage (.HitActor (Collision|BreakHitResult _outhit)) Damge 0 self))
    (:then_1
      (bind _newparam (CallFunction|Scatter (.Location (Collision|BreakHitResult _outhit)) false))
      (Effects|SpawnEmitteratLocation "/Game/BlockBreaker/ParticleSystems/PS_BulletImpact.PS_BulletImpact" _newparam)
      (Game|Damage|ApplyDamage 0 0.0 0 self))
    (:then_2
      (bind _newparam_2 (CallFunction|Scatter (.Location (Collision|BreakHitResult _outhit)) false))
      (Effects|SpawnEmitteratLocation "/Game/BlockBreaker/ParticleSystems/PS_BulletImpact.PS_BulletImpact" _newparam_2)
      (Game|Damage|ApplyDamage 0 0.0 0 self))
    (:then_3
      (bind _newparam_3 (CallFunction|Scatter (.Location (Collision|BreakHitResult _outhit)) false))
      (Effects|SpawnEmitteratLocation "/Game/BlockBreaker/ParticleSystems/PS_BulletImpact.PS_BulletImpact" _newparam_3)
      (Game|Damage|ApplyDamage 0 0.0 0 self))))

(fn Scatter
  (params (Location :type Vector) (Bool :type Boolean))
  (return (Math|Vector|RotateVectorAroundAxis "100.000000,10.000000, 0" (Math|Random|RandomFloatinRange 0.0 3.6e+02) Location)))